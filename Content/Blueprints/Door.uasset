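; Key-locked door actor that the player opens with Interact while inside its trigger volume.
; Trigger overlap enables and disables the actor's input, so Interact only works nearby.
; Interacting consumes one of the PlayerCharacter's keys and adds a key mesh at runtime, snapped to the KeyHole.
; The DoorOpening timeline then moves the key along local Y and the door mesh along Z.
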(event `self.TriggerVolume.OnComponentBeginOverlap`
  (params (OverlappedComponent :type "PrimitiveComponent Object Reference") (OtherActor :type "Actor Object Reference") (OtherComp :type "PrimitiveComponent Object Reference") (OtherBodyIndex :type Integer) (bFromSweep :type Boolean) (SweepResult :type "HitResult Structure (by ref)"))
  (if (== OtherActor (`GameplayStatics.GetPlayerCharacter` 0))
    (`self.EnableInput` (`GameplayStatics.GetPlayerController` 0))))

(event `InputAction|Interact`
  (params (Key :type "Key Structure"))
  (:`Pressed`
    (bind _asplayer_character (cast `/Game/Player/PlayerCharacter` (`GameplayStatics.GetPlayerCharacter` 0)))
    (bind _numberofkeys (`/Game/Player/PlayerCharacter.NumberOfKeys` _asplayer_character))
    (if (> _numberofkeys 0)
      (`/Engine/EditorBlueprintResources/StandardMacros.DecrementInt` _numberofkeys
        (:`  `
          (bind _returnvalue (`AddComponent|NODE_AddStaticMeshComponent-0`))
          (bind _output_get (set `self.KeyMesh` _returnvalue))
          (`SceneComponent.K2_AttachToComponent` _output_get (`self.KeyHole`) "None" "SnapToTarget" "SnapToTarget" "SnapToTarget" true)
          (bind (_direction _doorposition _keyposition) (`Timeline|DoorOpening` :!via `PlayFromStart`)
            (:`Update`
              (`SceneComponent.K2_SetRelativeLocation` (`self.KeyMesh`) (`KismetMathLibrary.MakeVector` 0.0 _keyposition) false false)
              (`SceneComponent.K2_SetRelativeLocation` (`self.DoorMesh`) (`KismetMathLibrary.MakeVector` 0.0 0.0 _doorposition) false false))))))))

(event `self.TriggerVolume.OnComponentEndOverlap`
  (params (OverlappedComponent :type "PrimitiveComponent Object Reference") (OtherActor :type "Actor Object Reference") (OtherComp :type "PrimitiveComponent Object Reference") (OtherBodyIndex :type Integer))
  (if (== OtherActor (`GameplayStatics.GetPlayerCharacter` 0))
    (`self.DisableInput` (`GameplayStatics.GetPlayerController` 0))))

(fn `UserConstructionScript`)